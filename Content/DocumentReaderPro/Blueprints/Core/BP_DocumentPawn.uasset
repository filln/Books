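; Input pawn for viewing documents, relaying player controls to a DocumentActor and its widget.
; Read, back, zoom and flip actions pass through actor-owned cooldown checks, with read and zoom also limited to the Inspection state.
; Axis input pans the cine camera while Zooming, smoothed except for mouse, and movement axes scroll text while Reading.
; Key presses and mouse movement report input device changes to the actor.
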(event Input|ActionEvents|InputActionDocumentRead
  (params (Key :type Key%20Structure))
  ;[1 1 1] Document Input Actions
  (:Pressed
    (Utilities|StartInputCooldown)
    (Utilities|OnlyWhileInspecting)
    (Default|OnReadDocument (Variables|Default|GetDocumentActor))))

(event Input|ActionEvents|InputActionDocumentFlip
  (params (Key :type Key%20Structure))
  ;[1 1 1] Document Input Actions
  (:Pressed
    (Utilities|StartFlipCooldown)
    (Default|OnFlipDocument (Variables|Default|GetDocumentActor))))

(event Input|ActionEvents|InputActionDocumentZoom
  (params (Key :type Key%20Structure))
  ;[1 1 1] Document Input Actions
  (:Pressed
    (Utilities|StartInputCooldown)
    (Utilities|OnlyWhileInspecting)
    (Default|OnZoomDocument (Variables|Default|GetDocumentActor))))

(event Input|ActionEvents|InputActionDocumentBack
  (params (Key :type Key%20Structure))
  ;[1 1 1] Document Input Actions
  (:Pressed
    (Utilities|StartInputCooldown)
    (Default|BackNavigation (Variables|/Game/DocumentReaderPro/Blueprints/Core/BP_DocumentActor_Custom.BP_DocumentActor_Custom_C|GetDocumentWidget (Variables|Default|GetDocumentActor)))))

(event Input|AxisEvents|InputAxisLookUp
  (params (AxisValue :type Float%20%28single-precision%29))
  ;[1 1 1] Camera Panning
  (Utilities|GreaterThanThreshold AxisValue 0.0)
  (Default|OnInputDeviceChanged (Variables|Default|GetDocumentActor) "NewEnumerator0")
  (Utilities|ExecuteState
    (:Zooming
      (Default|PanCineCam (Variables|Default|GetDocumentActor) (* AxisValue 0.2) (* (* (stale Input|AxisEvents|InputAxisTurn AxisValue) 0.2) -1.0) false))))

(event Input|AxisEvents|InputAxisTurnRate
  (params (AxisValue :type Float%20%28single-precision%29))
  ;[1 1 1] Camera Panning
  (Utilities|GreaterThanThreshold AxisValue 0.0)
  (Utilities|ExecuteState
    (:Zooming
      (Default|PanCineCam (Variables|Default|GetDocumentActor) (* AxisValue 0.1) (* (stale Input|AxisEvents|InputAxisLookUpRate AxisValue) 0.1) true))))

(event Input|AxisEvents|InputAxisTurn
  (params (AxisValue :type Float%20%28single-precision%29))
  ;[1 1 1] Camera Panning
  (Utilities|GreaterThanThreshold AxisValue 0.0)
  (Default|OnInputDeviceChanged (Variables|Default|GetDocumentActor) "NewEnumerator0")
  (Utilities|ExecuteState
    (:Zooming
      (Default|PanCineCam (Variables|Default|GetDocumentActor) (* (stale Input|AxisEvents|InputAxisLookUp AxisValue) 0.2) (* (* AxisValue 0.2) -1.0) false))))

(event Input|AxisEvents|InputAxisLookUpRate
  (params (AxisValue :type Float%20%28single-precision%29))
  ;[1 1 1] Camera Panning
  (Utilities|GreaterThanThreshold AxisValue 0.0)
  (Utilities|ExecuteState
    (:Zooming
      (Default|PanCineCam (Variables|Default|GetDocumentActor) (* (stale Input|AxisEvents|InputAxisTurnRate AxisValue) 0.1) (* AxisValue 0.1) true))))

(event Input|AxisEvents|InputAxisMoveForward
  (params (AxisValue :type Float%20%28single-precision%29))
  ;[1 1 1] Camera Panning
  (Utilities|GreaterThanThreshold AxisValue 0.0)
  (Utilities|ExecuteState
    (:Zooming
      (Default|PanCineCam (Variables|Default|GetDocumentActor) (* AxisValue 0.1) (* (stale Input|AxisEvents|InputAxisMoveRight AxisValue) 0.1) true))
    (:Reading
      (Default|UpdateScrollBoxPosition (Variables|/Game/DocumentReaderPro/Blueprints/Core/BP_DocumentActor_Custom.BP_DocumentActor_Custom_C|GetDocumentWidget (Variables|Default|GetDocumentActor)) AxisValue))))

(event Input|AxisEvents|InputAxisMoveRight
  (params (AxisValue :type Float%20%28single-precision%29))
  ;[1 1 1] Camera Panning
  (Utilities|GreaterThanThreshold AxisValue 0.0)
  (Utilities|ExecuteState
    (:Zooming
      (Default|PanCineCam (Variables|Default|GetDocumentActor) (* (stale Input|AxisEvents|InputAxisMoveForward AxisValue) 0.1) (* AxisValue 0.1) true))
    (:Reading
      (Default|UpdateScrollBoxPosition (Variables|/Game/DocumentReaderPro/Blueprints/Core/BP_DocumentActor_Custom.BP_DocumentActor_Custom_C|GetDocumentWidget (Variables|Default|GetDocumentActor)) (stale Input|AxisEvents|InputAxisMoveForward AxisValue)))))

(event Input|KeyboardEvents|AnyKey
  (params (Key :type Key%20Structure))
  ;[1 1 1] Detect Input Device Changes
  (:Pressed
    (if (or (Class|KismetInputLibrary|KeyIsKeyboardKey Key) (Class|KismetInputLibrary|KeyIsMouseButton Key))
      (Default|OnInputDeviceChanged (Variables|Default|GetDocumentActor) "NewEnumerator0")
      (else
        (Default|OnInputDeviceChanged (Variables|Default|GetDocumentActor) "NewEnumerator1")))))

(fn ConstructionScript)